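; AI controller for the Ripper enemy that sets up its blackboard on possession.
; The Possess event applies BB_Ripper, then seeds RipperState from the Ripper character and sets PlayerLocation to the zero vector.
; Tick is empty and a player-location lookup is left unconnected, so the controller neither updates those keys afterward nor starts a behavior tree.
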(event EventTick
  (params (DeltaSeconds :type Float%20%28single-precision%29)))

(event EventPossess
  (params (PossessedPawn :type Pawn%20Object%20Reference))
  (Class|AIController|UseBlackboard "/Game/_Game/Enemies/Ripper/BB_Ripper.BB_Ripper")
  (AI|Components|Blackboard|SetValueasEnum (Variables|Default|GetBlackboard) (Utilities|Name|MakeLiteralName "RipperState") (Variables|/Script/ProjectShock.PS_Ripper|GetRipperState (Variables|Default|GetRipperCharacter)))
  (AI|Components|Blackboard|SetValueasVector (Variables|Default|GetBlackboard) (Utilities|Name|MakeLiteralName "PlayerLocation") "0, 0, 0"))

(fn ConstructionScript)