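; Ripper enemy Blueprint that supports painting hits onto its skeletal mesh through a UV-unwrap scene capture.
; On BeginPlay it writes capture size and unwrap location to MPC_Global, clears RT_Capture after a short delay and creates a dynamic unwrap material.
; PaintActor briefly swaps that material onto the mesh, feeds it hit location and brush radius, captures the scene, then restores the original material.
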(event EventBeginPlay
  (Utilities|InitializeParameters
    (:Out
      (bind _returnvalue (Rendering|Material|CreateDynamicMaterialInstance "/Game/MeshPainter/Materials/EX_M_Unwrap.EX_M_Unwrap" "None" "Transient" :!class /Script/Engine.KismetMaterialLibrary))
      (Variables|Default|SetUnwrapMaterial _returnvalue))))

(event Collision|EventActorBeginOverlap
  (params (OtherActor :type Actor%20Object%20Reference)))

(event EventTick
  (params (DeltaSeconds :type Float%20%28single-precision%29)))

(fn ConstructionScript)

(fn PaintActor
  (params (HitLocation :type Vector) (BrushRadius :type Float%20%28single-precision%29))
  (Utilities|FlowControl|Sequence
    (:then_0
      (LocalVariables|SetOriginalMaterial (Rendering|Material|GetMaterial (Variables|Default|GetSkeletalMesh) 0))
      (Rendering|Material|SetMaterial (Variables|Default|GetSkeletalMesh) 0 (Variables|Default|GetUnwrapMaterial)))
    (:then_1
      (Rendering|Material|SetVectorParameterValue (Variables|Default|GetUnwrapMaterial) "HitLocation" (Math|Conversions|ToLinearColor(Vector) HitLocation) :!class /Script/Engine.MaterialInstanceDynamic)
      (Rendering|Material|SetScalarParameterValue (Variables|Default|GetUnwrapMaterial) "BrushRadius" BrushRadius :!class /Script/Engine.MaterialInstanceDynamic))
    (:then_2
      (Rendering|SceneCapture|CaptureScene (Variables|Default|GetSceneCapture) :!class /Script/Engine.SceneCaptureComponent2D)
      (Rendering|Material|SetMaterial (Variables|Default|GetSkeletalMesh) 0 (LocalVariables|GetOriginalMaterial)))))