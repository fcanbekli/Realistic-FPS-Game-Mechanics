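; Player controller that turns gamepad input into movement, look, aiming, sprinting and Glock equip/unequip on BP_Player.
; BeginPlay caches the pawn and its AnimBP_Player, which Tick feeds with axis values, debug-printing one.
; Left trigger sets aiming and plays or reverses a camera FOV timeline.
; D-pad montages set the active weapon, two keyboard keys trigger test-style montages, and walk-speed and rotation nodes are left unconnected.
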(event EventBeginPlay
  (bind _asbp_player (Utilities|Casting|CastToBP_Player (Game|Player|GetPlayerPawn 0)))
  (Variables|Default|SetPlayerCharacter _asbp_player)
  (bind _asanim_bp_player (Utilities|Casting|CastToAnimBP_Player (Components|SkeletalMesh|GetAnimInstance (Variables|/Script/Engine.Character|GetMesh (Variables|Default|GetPlayerCharacter)))))
  (Variables|Default|SetAnimationBlueprint _asanim_bp_player))

(event EventTick
  (params (DeltaSeconds :type Float%20%28single-precision%29))
  (bind _animationblueprint (Variables|Default|GetAnimationBlueprint))
  (Variables|/Script/ProjectShock.PS_PlayerAnimation|SetXAxisValue _animationblueprint (Class|Actor|GetInputAxisKeyValue))
  (bind _output_get (Variables|/Script/ProjectShock.PS_PlayerAnimation|SetXRightAxisValue _animationblueprint (Class|Actor|GetInputAxisKeyValue)))
  (Development|PrintString (Utilities|String|ToString(Float) _output_get)))

(event Input|GamepadEvents|GamepadLeftX
  (params (AxisValue :type Float%20%28single-precision%29))
  (Class|PSPlayerController|MoveSide AxisValue))

(event Input|GamepadEvents|GamepadLeftY
  (params (AxisValue :type Float%20%28single-precision%29))
  (Class|PSPlayerController|MoveForward AxisValue))

(event Input|GamepadEvents|GamepadRightX
  (params (AxisValue :type Float%20%28single-precision%29))
  (Class|PSPlayerController|TurnMovement AxisValue))

(event Input|GamepadEvents|GamepadRightY
  (params (AxisValue :type Float%20%28single-precision%29))
  (Class|PSPlayerController|LoopUpMovement AxisValue))

(event Input|GamepadEvents|GamepadRightTrigger
  (params (Key :type Key%20Structure :default "None")))

(event Input|GamepadEvents|GamepadLeftTrigger
  (params (Key :type Key%20Structure :default "None"))
  (bind _playercharacter (Variables|Default|GetPlayerCharacter))
  (:Pressed
    (Variables|/Script/ProjectShock.PS_PlayerCharacter|SetbIsAiming _playercharacter true)
    (bind _newtrack_0 (Timeline|Timeline_0 PlayFromStart)
      (:Update
        (Camera|SetFieldOfView (Variables|/Script/ProjectShock.PS_PlayerCharacter|GetFPS_Camera (Variables|Default|GetPlayerCharacter)) _newtrack_0))))
  (:Released
    (Variables|/Script/ProjectShock.PS_PlayerCharacter|SetbIsAiming _playercharacter false)
    (Timeline|Timeline_0 ReverseFromEnd)))

(event Input|GamepadEvents|GamepadFaceButtonRight
  (params (Key :type Key%20Structure :default "None")))

(event Input|KeyboardEvents|SpaceBar
  (params (Key :type Key%20Structure :default "None"))
  (:Pressed
    (Animation|Montage|PlayMontage (Variables|/Script/Engine.Character|GetMesh (Variables|Default|GetPlayerCharacter)) "/Game/_Game/Player/Animations/AM_Glock_Relaxing_Idle.AM_Glock_Relaxing_Idle" 0.7)))

(event Input|GamepadEvents|GamepadDPadLeft
  (params (Key :type Key%20Structure :default "None"))
  ;[1 1 1] Equip
  (:Pressed
    (Animation|Montage|PlayMontage (Variables|/Script/Engine.Character|GetMesh (Variables|Default|GetPlayerCharacter)) "/Game/_Game/Player/Animations/AM_Glock_Equip.AM_Glock_Equip"
      (:then
        (Variables|/Script/ProjectShock.PS_PlayerCharacter|SetActiveWeapon (Variables|Default|GetPlayerCharacter) "Glock")))))

(event Input|KeyboardEvents|3
  (params (Key :type Key%20Structure :default "None"))
  (:Pressed
    (Animation|Montage|PlayMontage (Variables|/Script/Engine.Character|GetMesh (Variables|Default|GetPlayerCharacter)) 0 1.5)))

(event Input|GamepadEvents|GamepadDPadRight
  (params (Key :type Key%20Structure :default "None"))
  ;[1 1 1] Unequip
  (:Pressed
    (Animation|Montage|PlayMontage (Variables|/Script/Engine.Character|GetMesh (Variables|Default|GetPlayerCharacter)) "/Game/_Game/Player/Animations/AM_Glock_Unequip.AM_Glock_Unequip"
      (:OnCompleted
        (Variables|/Script/ProjectShock.PS_PlayerCharacter|SetActiveWeapon (Variables|Default|GetPlayerCharacter) "Unarmed")))))

(event Input|GamepadEvents|GamepadLeftThumbstick
  (params (Key :type Key%20Structure :default "None"))
  (bind _playercharacter (Variables|Default|GetPlayerCharacter))
  (:Pressed
    (Variables|/Script/ProjectShock.PS_PlayerCharacter|SetbIsSprinting _playercharacter true))
  (:Released
    (Variables|/Script/ProjectShock.PS_PlayerCharacter|SetbIsSprinting _playercharacter false)))

(fn ConstructionScript)