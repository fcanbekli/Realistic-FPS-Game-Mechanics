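; Player camera manager that handles aim zoom in and out on the player's first-person camera.
; AimZoomIn and AimZoomOut each drive BP_Player's FPSCamera field of view with their own timeline, the first played forward from the start and the second reversed from the end.
; Each timeline update also sets the player's IsDeepAiming flag, true for zoom in and false for zoom out.
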(event Custom|AimZoomIn
  ;[1 1 1] Zoom In/Out
  (bind _asbp_player (Utilities|Casting|CastToBP_Player (Game|Player|GetPlayerPawn 0)))
  (bind _newtrack_0 (Timeline|Timeline_0 PlayFromStart)
    (:Update
      (Camera|SetFieldOfView (Variables|/Script/ProjectShock.PS_PlayerCharacter|GetFPS_Camera _asbp_player) _newtrack_0)
      (Variables|/Script/ProjectShock.PS_PlayerCharacter|SetbIsDeepAiming _asbp_player true))))

(event Custom|AimZoomOut
  ;[1 1 1] Zoom In/Out
  (bind _asbp_player (Utilities|Casting|CastToBP_Player (Game|Player|GetPlayerPawn 0)))
  (bind _newtrack_0 (Timeline|Timeline_1 ReverseFromEnd)
    (:Update
      (Camera|SetFieldOfView (Variables|/Script/ProjectShock.PS_PlayerCharacter|GetFPS_Camera _asbp_player) _newtrack_0)
      (Variables|/Script/ProjectShock.PS_PlayerCharacter|SetbIsDeepAiming _asbp_player false))))

(event EventBeginPlay)

(event Collision|EventActorBeginOverlap
  (params (OtherActor :type Actor%20Object%20Reference)))

(event EventTick
  (params (DeltaSeconds :type Float%20%28single-precision%29)))

(fn ConstructionScript)