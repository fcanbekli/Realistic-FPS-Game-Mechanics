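; BP_Player is the player Blueprint, setting up a first-person camera, a weapon and a Cytosine child actor on BeginPlay.
; It spawns BP_DummyGun and BP_ElectricCytosine at the world origin, then passes their classes to the Weapon and Cytosine child actor components.
; The camera and weapon actor then snap to mesh sockets.
; A number-key press subtracts Health, with no clamp or death check here.
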(event EventBeginPlay
  (bind _returnvalue (Math|Conversions|ToTransform(Vector) "0, 0, 0"))
  (Utilities|FlowControl|Sequence
    (:then_0
      (bind _returnvalue_2 (Game|SpawnActorfromClass "/Game/_Game/Weapons/BP_DummyGun.BP_DummyGun_C" _returnvalue "Undefined" 0 0))
      (ChildActorComponent|SetChildActorClass (Variables|Default|GetWeapon) (Utilities|GetClass _returnvalue_2)))
    (:then_1
      (bind _returnvalue_3 (Game|SpawnActorfromClass "/Game/_Game/Cytosines/BP_ElectricCytosine.BP_ElectricCytosine_C" _returnvalue "Undefined" 0 0))
      (ChildActorComponent|SetChildActorClass (Variables|Default|GetCytosine) (Utilities|GetClass _returnvalue_3)))
    (:then_2
      (Transformation|AttachComponentToComponent (Variables|Default|GetFPS_Camera) (Variables|Character|GetMesh) "CameraSocket" "SnapToTarget" "SnapToTarget" "SnapToTarget" true)
      (Transformation|AttachComponentToComponent (Variables|/Script/Engine.ChildActorComponent|GetChildActor (Variables|Default|GetWeapon)) (Variables|Character|GetMesh) "WeaponSocket" "SnapToTarget" "SnapToTarget" "SnapToTarget" true))))

(event Collision|EventActorBeginOverlap
  (params (OtherActor :type Actor%20Object%20Reference)))

(event EventTick
  (params (DeltaSeconds :type Float%20%28single-precision%29)))

(event Input|KeyboardEvents|1
  (params (Key :type Key%20Structure :default "None"))
  (:Pressed
    (Variables|Default|SetHealth (- (Variables|Default|GetHealth) 1e+01))))

(fn ConstructionScript)