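; BP_HandgunAmmoBox is a handgun ammo loot object that hides its loot icon when the player comes close.
; Each Tick it measures the distance to the first player's pawn and prints it as debug output.
; Within a short range it calls FadeOut on the BP_LootIcon widget from its LootIconWidget component, repeating every frame.
; It contains no pickup or ammo-granting logic.
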(event EventBeginPlay)

(event Collision|EventActorBeginOverlap
  (params (OtherActor :type Actor%20Object%20Reference)))

(event EventTick
  (params (DeltaSeconds :type Float%20%28single-precision%29))
  (bind _returnvalue (Game|Player|GetPlayerPawn 0))
  (bind _returnvalue_2 (Transformation|GetActorTransform))
  (bind _location (Math|Transform|BreakTransform _returnvalue_2))
  (bind _returnvalue_3 (Transformation|GetActorTransform _returnvalue))
  (bind _location_2 (Math|Transform|BreakTransform _returnvalue_3))
  (bind _returnvalue_4 (- _location_2 _location))
  (bind _returnvalue_5 (Math|Vector|VectorLength _returnvalue_4))
  (Development|PrintString (Utilities|String|ToString(Float) _returnvalue_5))
  (if (< _returnvalue_5 2e+02)
    (bind _asbp_loot_icon (Utilities|Casting|CastToBP_LootIcon (UserInterface|GetWidget (Variables|Default|GetLootIconWidget))))
    (Class|PSLootIcon|FadeOut _asbp_loot_icon)))

(fn ConstructionScript)