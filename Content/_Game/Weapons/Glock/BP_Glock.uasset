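; Player Glock weapon Blueprint that handles firing and reloading.
; FireWeapon calls FireGlock, defined outside these graphs, then LineTrace casts a camera-forward ray and branches on physical surface, calling HitFunciton on hit enemies and only printing for wood.
; Reload plays empty or regular weapon montages alongside a player montage, refills the magazine immediately, flags reloading on BP_PlayerState and updates the HUD on completion.
; Older shooting, effects and decal logic remains disconnected.
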(event EventBeginPlay
  (Variables|Default|SetCurrentMagazineSize (Variables|Default|GetMaxMagazineSize)))

(event Collision|EventActorBeginOverlap
  (params (OtherActor :type Actor%20Object%20Reference)))

(event EventTick
  (params (DeltaSeconds :type Float%20%28single-precision%29)))

(event EventFireWeapon
  ;[1 1 1] Fire
  (Class|PSGlock|FireGlock)
  (CallFunction|LineTrace))

(event EventReload
  ;[1 1 1] Reloading
  (if (== (Variables|Default|GetCurrentMagazineSize) 0)
    (Animation|Montage|PlayMontage (Variables|Default|GetWeaponMesh) "/Game/_Game/Weapons/Glock/Animations/AM_Glock_Reloading_Empty.AM_Glock_Reloading_Empty"
      (:then
        _))
    (else
      (Animation|Montage|PlayMontage (Variables|Default|GetWeaponMesh) "/Game/_Game/Weapons/Glock/Animations/AM_GlockReload.AM_GlockReload"
        (:then
          _))))
  (bind _asbp_player (Utilities|Casting|CastToBP_Player (Game|Player|GetPlayerPawn 0)))
  (Animation|Montage|PlayMontage (Variables|/Script/Engine.Character|GetMesh _asbp_player) "/Game/_Game/Player/Animations/AM_GlockScottReload.AM_GlockScottReload"
    (:then
      (Variables|Default|SetCurrentMagazineSize (Variables|Default|GetMaxMagazineSize))
      (bind _asbp_player_state (Utilities|Casting|CastToBP_PlayerState (Variables|/Script/Engine.Pawn|GetPlayerState (Game|GetPlayerCharacter 0))))
      (Variables|/Script/ProjectShock.PS_PlayerState|SetbIsReloding _asbp_player_state true))
    (:OnCompleted
      (bind _asbp_hud (Utilities|Casting|CastToBP_HUD (HUD|GetHUD (Game|GetPlayerController 0))))
      (Class|PSHUD|UpdateAmmoBar _asbp_hud))))

(fn ConstructionScript)

(fn LineTrace
  (bind _asbp_player (Utilities|Casting|CastToBP_Player (Game|Player|GetPlayerPawn 0)))
  (Utilities|Casting|CastToBP_HUD (HUD|GetHUD (Game|GetPlayerController 0)))
  (bind _outhit (Collision|LineTraceByChannel (Transformation|GetWorldLocation (Variables|/Script/ProjectShock.PS_PlayerCharacter|GetFPS_Camera _asbp_player)) (+ (Transformation|GetWorldLocation (Variables|/Script/ProjectShock.PS_PlayerCharacter|GetFPS_Camera _asbp_player)) (* (Math|Vector|GetForwardVector (Transformation|GetWorldRotation (Variables|/Script/ProjectShock.PS_PlayerCharacter|GetFPS_Camera _asbp_player))) "1500.000000,1500.000000,1500.000000")) "TraceTypeQuery1" true 0 "None" true "(R=1.000000,G=0.000000,B=0.000000,A=1.000000)" "(R=0.000000,G=1.000000,B=0.000000,A=1.000000)" 2.0))
  (switch Utilities|FlowControl|Switch|SwitchonEPhysicalSurface (Variables|/Script/PhysicsCore.PhysicalMaterial|GetSurfaceType (.PhysMat (Collision|BreakHitResult _outhit)))
    (:SurfaceType1
      (Development|PrintString "Wood"))
    (:SurfaceType2
      ;[1 1 1] Base Enemy
      (bind _asps_base_enemy (Utilities|Casting|CastToPS_BaseEnemy (.HitActor (Collision|BreakHitResult _outhit))))
      (Class|PSBaseEnemy|HitFunciton _asps_base_enemy))))